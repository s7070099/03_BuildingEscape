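; Openable door actor that swings open and closed when its OpenDoor component fires open and close events.
; BeginPlay stores the initial rotation, and a DoorSwing timeline adds its OpenAngle curve as yaw on top of it each update.
; A timeline event track triggers the door lock sound at the actor's location, and closing simply reverses the timeline.
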(event `self.ReceiveBeginPlay`
  (set `self.Init Rotation` (`self.K2_GetActorRotation`)))

(event `self.OpenDoor.OnOpen`
  (bind (_direction _open_angle) (`Timeline|Door Swing` :!label _label)
    (:`Update`
      (`self.K2_SetActorRotation` (`KismetMathLibrary.ComposeRotators` (`KismetMathLibrary.MakeRotator` 0.0 0.0 _open_angle) (`self.Init Rotation`))))
    (:`Sound Timer`
      (`GameplayStatics.PlaySoundAtLocation` "/Game/Audio/door-lock.door-lock" (`self.K2_GetActorLocation`)))))

(event `self.OpenDoor.OnClose`
  (goto _label :!via `Reverse`))

(fn `UserConstructionScript`)